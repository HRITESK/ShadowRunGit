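; BP_Slime is a PaperZD slime enemy that dies to any damage and awards score to the player.
; Jumps in the Locomotion state machine play attack and death animations; the actor is destroyed when the attack ends or after a death delay.
; BeginPlay caches the player and health bar widget, which empties on damage.
; Getter functions expose its damage, self reference and spline path, while Tick fires an attack-end dispatcher once flagged.
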(event Custom|Attack01
  (if (not (Variables|Default|GetISDead?))
    (Utilities|FlowControl|Delay 0.6)
    (Variables|Default|SetIsAttackEnd false)
    (Utilities|IsValid self
      (:Is%20Valid
        (Class|PaperZDAnimInstance|JumptoNode (Variables|/Script/PaperZD.PaperZDAnimationComponent|GetAnimInstance (Variables|Default|GetAnimationComponent)) "Attack01" "Locomotion")))))

(event Custom|Attack01End
  (params (IsAttackEnd :type Boolean))
  (Variables|Default|SetIsAttackEnd IsAttackEnd)
  (Actor|DestroyActor self))

(event Game|Damage|EventAnyDamage
  (params (Damage :type Float%20%28single-precision%29) (DamageType :type Damage%20Type%20Object%20Reference) (InstigatedBy :type Controller%20Object%20Reference) (DamageCauser :type Actor%20Object%20Reference))
  (bind _bp_player (Variables|Default|GetBP_Player))
  (CallFunction|HealthWidgetUpdate 0.0)
  (Variables|Default|SetISDead? true)
  (Class|PaperZDAnimInstance|JumptoNode (Variables|/Script/PaperZD.PaperZDAnimationComponent|GetAnimInstance (Variables|Default|GetAnimationComponent)) "Death" "Locomotion")
  (Utilities|FlowControl|Delay 0.6)
  (Actor|DestroyActor)
  (Variables|/Game/Assets/PaperZD/BP_PaperZDCharacter.BP_PaperZDCharacter_C|SetScore _bp_player (+ (Variables|/Game/Assets/PaperZD/BP_PaperZDCharacter.BP_PaperZDCharacter_C|GetScore _bp_player) 5e+01)))

(event EventBeginPlay
  ;[1 1 1] Begin
  (bind _asbp_paper_zdcharacter (Utilities|Casting|CastToBP_PaperZDCharacter (Game|GetPlayerCharacter 0)))
  (Variables|Default|SetBP_Player _asbp_paper_zdcharacter)
  (Variables|Default|SetISDead? false)
  (bind _aswbp_enemy_health (Utilities|Casting|CastToWBP_EnemyHealth (UserInterface|GetWidget (Variables|Default|GetHealthBar))))
  (Variables|Default|SetWBP%20Enemy%20Health%20Instance _aswbp_enemy_health)
  (CallFunction|HealthWidgetUpdate 1e+02))

(event EventTick
  (params (DeltaSeconds :type Float%20%28single-precision%29))
  (if (Variables|Default|GetIsAttackEnd)
    (Default|CallAttackEnddispatcher)))

(fn ConstructionScript)

(fn HealthWidgetUpdate
  (params (Percent :type Float%20%28single-precision%29))
  (Progress|SetPercent (Variables|/Game/Assets/Widger/WBP_EnemyHealth.WBP_EnemyHealth_C|GetHealthBar (Variables|Default|GetWBP%20Enemy%20Health%20Instance)) Percent))

(fn SendDamage
  (return 5e+01))

(fn SendEnemyPaper
  (return self))

(fn SendSplineObject
  (return (Variables|Default|GetSplinePath)))