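; PaperZD enemy character with health, an attack, a health bar widget and a score reward on death.
; AnyDamage lowers health, and Attack01 jumps the Locomotion state machine to its attack node while health is positive.
; Tick calls the attack-end dispatcher and refreshes the bar when not attacking; below zero health it awards score once, plays Death and destroys the actor.
; Getters expose damage, self and spline path.
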(event Custom|Attack01
  ;[0.5189 0 1 1 30] AttackEvent
  (if (> (Variables|Character|GetEnemyHealth) 0)
    (Variables|Character|SetIsAttackEnd false)
    (Class|PaperZDAnimInstance|JumptoNode (Variables|/Script/PaperZD.PaperZDAnimationComponent|GetAnimInstance (Variables|Default|GetAnimationComponent)) "Attack01" "Locomotion")))

(event Custom|Attack01End
  (params (IsAttackEnd :type Boolean))
  ;[0.5189 0 1 1 30] AttackEvent
  (Variables|Character|SetIsAttackEnd IsAttackEnd))

(event Game|Damage|EventAnyDamage
  (params (Damage :type Float%20%28single-precision%29) (DamageType :type Damage%20Type%20Object%20Reference) (InstigatedBy :type Controller%20Object%20Reference) (DamageCauser :type Actor%20Object%20Reference))
  ;[1 0 0.06124 0.671 30] take Damage
  (Variables|Character|SetEnemyHealth (Math|Float|Truncate (- (Variables|Character|GetEnemyHealth) Damage))))

(event EventBeginPlay
  ;[0 0 0 1 30] Begin
  (bind _asbp_paper_zdcharacter (Utilities|Casting|CastToBP_PaperZDCharacter (Game|GetPlayerCharacter 0)))
  (Variables|Instance|SetBP_player _asbp_paper_zdcharacter)
  (bind _aswbp_enemy_health (Utilities|Casting|CastToWBP_EnemyHealth (UserInterface|GetWidget (Variables|Default|GetHealthBar))))
  (Variables|Instance|SetWBP%20Enemy%20Health%20Instance _aswbp_enemy_health)
  (CallFunction|SetHealthBarPercentage))

(event EventTick
  (params (DeltaSeconds :type Float%20%28single-precision%29))
  (bind _bp_player (Variables|Instance|GetBP_player))
  ;[0.4217 0 1 0.358 30] Tick
  (if (< (Variables|Character|GetEnemyHealth) 0)
    (Utilities|FlowControl|DoOnce false
      (:Completed
        (Variables|/Game/Assets/PaperZD/BP_PaperZDCharacter.BP_PaperZDCharacter_C|SetScore _bp_player (+ (Variables|/Game/Assets/PaperZD/BP_PaperZDCharacter.BP_PaperZDCharacter_C|GetScore _bp_player) 1e+02))
        (Class|PaperZDAnimInstance|JumptoNode (Variables|/Script/PaperZD.PaperZDAnimationComponent|GetAnimInstance (Variables|Default|GetAnimationComponent)) "Death" "Locomotion")
        (Utilities|FlowControl|Delay 2.0)
        (Actor|DestroyActor)
        (CallFunction|SetHealthBarPercentage)))
    (elif (Variables|Character|GetIsAttackEnd)
      (Default|CallAttackEnddispatcher)
      (CallFunction|SetHealthBarPercentage))))

(fn ConstructionScript)

(fn SetHealthBarPercentage
  (Progress|SetPercent (Variables|/Game/Assets/Widger/WBP_EnemyHealth.WBP_EnemyHealth_C|GetHealthBar (Variables|Instance|GetWBP%20Enemy%20Health%20Instance)) (/ (Math|Conversions|ToFloat(Integer) (Variables|Character|GetEnemyHealth)) 1e+02)))

(fn SendDamage
  (return 2e+01))

(fn SendEnemyPaper
  (return self))

(fn SendSplineObject
  (return (Variables|Instance|GetSplinePath)))