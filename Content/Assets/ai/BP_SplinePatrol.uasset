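; BP_SplinePatrol is a patrol route that uses a spline's points as waypoints, apparently for AI.
; IncrementSplinePoint steps CurrentPoint along the spline, flipping Direction at the last and first points so the route ping-pongs rather than loops.
; GetSplineWorldPosition returns the current point's world location.
; The blueprint only tracks the waypoint and moves nothing itself.
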(event Custom|IncrementSplinePoint
  (bind _output_get (Variables|Default|SetCurrentPoint (+ (Variables|Default|GetCurrentPoint) (Variables|Default|GetDirection))))
  (if (== _output_get (- (Spline|GetNumberOfSplinePoints (Variables|Default|GetSpline)) 1))
    (Variables|Default|SetDirection -1)
    (elif (== (Variables|Default|GetCurrentPoint) 0)
      (Variables|Default|SetDirection 1))))

(fn ConstructionScript)

(fn GetSplineWorldPosition
  (return (Spline|GetLocationatSplinePoint (Variables|Default|GetSpline) (Variables|Default|GetCurrentPoint) "World")))