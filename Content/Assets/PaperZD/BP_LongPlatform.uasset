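; BP_LongPlatform is a platform actor whose Box1 component periodically moves vertically and back.
; BeginPlay starts a looping three-second timer that replays the 0To1To0 timeline from the start.
; The timeline lerps Box1's relative location between the origin and the Z part of Offset without sweeping, and EndPlay clears the timer.
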(event Custom|Start%20Oscilating
  (bind _newtrack_0 (Timeline|0%20to%201%20to%200 PlayFromStart)
    (:Update
      (Transformation|SetRelativeLocation (Variables|Default|GetBox1) (Math|Vector|Lerp(Vector) "0, 0, 0" (* (Variables|Default|GetOffset) "0.000000,0.000000,1.000000") _newtrack_0) false false))))

(event EventEndPlay
  (params (EndPlayReason :type EEndPlayReason%20Enum :default "Destroyed"))
  (Utilities|Time|ClearandInvalidateTimerbyHandle (Variables|Default|GetTimer)))

(event EventBeginPlay
  (bind _returnvalue (Utilities|Time|SetTimerbyEvent (delegate Custom|Start%20Oscilating) 3.0 true))
  (Variables|Default|SetTimer _returnvalue))

(fn ConstructionScript)